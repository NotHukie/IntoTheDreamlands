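; Actor that scatters bubble-burst VFX over preset regions of the level at a fixed height.
; BeginPlay starts a fast looping timer on Fx, which tests random Y-band checks to choose X ranges, then spawns FX_BubleBurst at random scale.
; Each check and the final Y are rolled independently, so Y is not tied to the chosen band and some ticks spawn nothing.
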(event `Fx`
  (bind _returnvalue (`KismetMathLibrary.RandomFloatInRange` 1620.0 7800.0))
  (if (and (<= _returnvalue 7800.0) (>= _returnvalue 6000.0))
    (set `self.Y` _returnvalue)
    (if (== (`KismetMathLibrary.RandomInteger` 1) 0)
      (set `self.X` (`KismetMathLibrary.RandomFloatInRange` -2500.0 -1300.0))
      (else
        (set `self.X` (`KismetMathLibrary.RandomFloatInRange` 3250.0 4500.0))))
    (`NiagaraFunctionLibrary.SpawnSystemAtLocation` "/Game/Assets/VFX/BubleBurst/FX_BubleBurst.FX_BubleBurst" (`KismetMathLibrary.MakeVector` (`self.X`) (`self.Y`) 900.0) (struct) (`KismetMathLibrary.Conv_DoubleToVector` (`KismetMathLibrary.RandomFloatInRange` 0.5 1.0)) :!label _label)
    (elif (and (<= _returnvalue 5980.0) (>= _returnvalue 4000.0))
      (set `self.Y` _returnvalue)
      (if (== (`KismetMathLibrary.RandomInteger` 1) 0)
        (set `self.X` (`KismetMathLibrary.RandomFloatInRange` -1090.0 2900.0))
        (goto _label)
        (else
          (set `self.X` (`KismetMathLibrary.RandomFloatInRange` -2500.0 -1300.0))
          (goto _label)))
      (elif (and (<= _returnvalue 3840.0) (>= _returnvalue 2600.0))
        (set `self.Y` _returnvalue)
        (if (== (`KismetMathLibrary.RandomInteger` 1) 0)
          (set `self.X` (`KismetMathLibrary.RandomFloatInRange` -1090.0 -470.0))
          (goto _label)
          (else
            (set `self.X` (`KismetMathLibrary.RandomFloatInRange` -2500.0 -1300.0))
            (goto _label)))
        (elif (and (<= _returnvalue 2580.0) (>= _returnvalue 1620.0))
          (set `self.Y` _returnvalue)
          (switch `int` (`KismetMathLibrary.RandomInteger` 2)
            (:`0`
              (set `self.X` (`KismetMathLibrary.RandomFloatInRange` -1090.0 -470.0))
              (goto _label))
            (:`1`
              (set `self.X` (`KismetMathLibrary.RandomFloatInRange` -2500.0 -1300.0))
              (goto _label))
            (:`2`
              (set `self.X` (`KismetMathLibrary.RandomFloatInRange` 1540.0 2840.0))
              (goto _label))))))))

(event `self.ReceiveBeginPlay`
  (`KismetSystemLibrary.K2_SetTimer` null "Fx" 0.1 true))

(fn `UserConstructionScript`)
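; BP_BubleSpawnJets is an effect spawner that continuously places bubble burst jets across a fixed area of the level.
; On BeginPlay, a fast looping timer calls the Fx event.
; Each call spawns the FX_BubleBurst system at a random X and Y within hardcoded world bounds, at a constant height and with a random uniform scale.
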(event `Fx`
  (set `self.Y` (`KismetMathLibrary.RandomFloatInRange` -2463.0 7355.0))
  (set `self.X` (`KismetMathLibrary.RandomFloatInRange` 5733.0 7355.0))
  (`NiagaraFunctionLibrary.SpawnSystemAtLocation` "/Game/Assets/VFX/BubleBurst/FX_BubleBurst.FX_BubleBurst" (`KismetMathLibrary.MakeVector` (`self.X`) (`self.Y`) 1850.0) (struct) (`KismetMathLibrary.Conv_DoubleToVector` (`KismetMathLibrary.RandomFloatInRange` 0.5 1.0))))

(event `self.ReceiveBeginPlay`
  (`KismetSystemLibrary.K2_SetTimer` null "Fx" 0.1 true))

(fn `UserConstructionScript`)
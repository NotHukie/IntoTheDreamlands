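; BP_ShaderGate is a two-part gate visual that fades or fills each side through a shader parameter.
; On BeginPlay it gives its two plane meshes separate dynamic instances of M_Gate, one tinted orange-red and the other blue.
; GateSara and GateTomas events each play or reverse their own timeline, which drives the Percentage parameter of the matching plane's material.
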(event `self.ReceiveBeginPlay`
  (bind _shadergateplanes (`self.ShaderGatePlanes`))
  (bind _output_get (set `self.Areas` (`|MakeArray` _shadergateplanes (`self.ShaderGatePlanes2`))))
  (for _array_element _output_get
    (if (== _array_element _shadergateplanes)
      (bind _returnvalue (`PrimitiveComponent.CreateDynamicMaterialInstance` _array_element 0 "/Game/Assets/Shaders/Gate/M_Gate.M_Gate" "None"))
      (bind _output_get_2 (set `self.NewMaterialInstance` _returnvalue))
      (`MaterialInstanceDynamic.SetVectorParameterValue` _output_get_2 "Color" (struct :`R` 0.911458 :`G` 0.231829 :`B` 0.071208 :`A` 1.0))
      (`PrimitiveComponent.SetMaterial` _array_element 0 _output_get_2)
      (else
        (bind _returnvalue_2 (`PrimitiveComponent.CreateDynamicMaterialInstance` _array_element 0 "/Game/Assets/Shaders/Gate/M_Gate.M_Gate" "None"))
        (bind _output_get_3 (set `self.NewMaterialInst2` _returnvalue_2))
        (`MaterialInstanceDynamic.SetVectorParameterValue` _output_get_3 "Color" (struct :`R` 0.224051 :`G` 0.253753 :`B` 0.911458 :`A` 1.0))
        (`PrimitiveComponent.SetMaterial` _array_element 0 _output_get_3)))))

(event `GateSara`
  (params (reverse :type Boolean))
  (if (not reverse)
    (bind (_direction _newtrack_0) (`Timeline|Timeline_0` :!label _label)
      (:`Update`
        (`MaterialInstanceDynamic.SetScalarParameterValue` (`self.NewMaterialInstance`) "Percentage" _newtrack_0)))
    (else
      (goto _label :!via `Reverse`))))

(event `GateTomas`
  (params (reverse :type Boolean))
  (if (not reverse)
    (bind (_direction _newtrack_0) (`Timeline|Timeline_1` :!label _label_2)
      (:`Update`
        (`MaterialInstanceDynamic.SetScalarParameterValue` (`self.NewMaterialInst2`) "Percentage" _newtrack_0)))
    (else
      (goto _label_2 :!via `Reverse`))))

(fn `UserConstructionScript`)
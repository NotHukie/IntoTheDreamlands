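; BP_PortalManager is an actor that provides the math for mapping locations, directions, rotations and velocities from one portal's space into another's.
; Locations use a current-portal transform with negated X and Y scale, while a mirrored variant negates only Y.
; Directions are mirrored across local X and Y, and feed rotation (rebuilt from two axes) and velocity (magnitude preserved).
; Tick only converts the target portal's location and discards the result.
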(event `self.ReceiveTick`
  (params (DeltaSeconds :type "Float (single-precision)"))
  (bind _targetportal (`self.TargetPortal`))
  (bind _returnvalue_location (`KismetMathLibrary.BreakTransform` (`self.GetTransform` _targetportal)))
  (`self.PortalConvertLocation` (`self.CurrentPortal`) _targetportal _returnvalue_location))

(fn `PortalConvertDirection`
  (params (CurrentPortal :type "Actor Object Reference") (TargetPortal :type "Actor Object Reference") (PrevDirection :type "Vector Structure"))
  (returns (NewDirection :type "Vector Structure"))
  (bind _output_get (set `self.Direction` (`KismetMathLibrary.TransformDirection` (`self.GetTransform` TargetPortal) (`KismetMathLibrary.MirrorVectorByNormal` (`KismetMathLibrary.MirrorVectorByNormal` (`KismetMathLibrary.InverseTransformDirection` (`self.GetTransform` CurrentPortal) PrevDirection) (1.0 0.0 0.0)) (0.0 1.0 0.0)))))
  (return _output_get))

(fn `PortalConvertLocation`
  (params (CurrentPortal :type "Actor Object Reference") (TargetPortal :type "Actor Object Reference") (PrevLocation :type "Vector Structure"))
  (returns (NewLocation :type "Vector Structure"))
  (bind _output_get (set `self.Location` (`KismetMathLibrary.TransformLocation` (`self.GetTransform` TargetPortal) (`KismetMathLibrary.InverseTransformLocation` (`KismetMathLibrary.MakeTransform` (.location (`self.GetTransform` CurrentPortal)) (.rotation (`self.GetTransform` CurrentPortal)) (`KismetMathLibrary.MakeVector` (* (.x (.scale (`self.GetTransform` CurrentPortal))) -1.0) (* (.y (.scale (`self.GetTransform` CurrentPortal))) -1.0) (.z (.scale (`self.GetTransform` CurrentPortal))))) PrevLocation))))
  (return _output_get))

(fn `PortalConvertLocationMirrored`
  (params (CurrentPortal :type "Actor Object Reference") (TragetPortal :type "Actor Object Reference") (PrevLocation :type "Vector Structure"))
  (returns (NewLocation :type "Vector Structure"))
  (bind _output_get (set `self.Location` (`KismetMathLibrary.TransformLocation` (`self.GetTransform` TragetPortal) (`KismetMathLibrary.InverseTransformLocation` (`KismetMathLibrary.MakeTransform` (.location (`self.GetTransform` CurrentPortal)) (.rotation (`self.GetTransform` CurrentPortal)) (`KismetMathLibrary.MakeVector` (.x (.scale (`self.GetTransform` CurrentPortal))) (* (.y (.scale (`self.GetTransform` CurrentPortal))) -1.0) (.z (.scale (`self.GetTransform` CurrentPortal))))) PrevLocation))))
  (return _output_get))

(fn `PortalConvertRotation`
  (params (CurrentPortal :type "Actor Object Reference") (rgetPortal :type "Actor Object Reference") (PrevRotation :type "Rotator Structure"))
  (returns (NewRotation :type "Rotator Structure"))
  (bind (_x _y) (`KismetMathLibrary.GetAxes` PrevRotation))
  (bind _newdirection (`self.PortalConvertDirection` CurrentPortal rgetPortal _x))
  (set `self.DrX` _newdirection)
  (bind _newdirection_2 (`self.PortalConvertDirection` CurrentPortal rgetPortal _y))
  (set `self.DrY` _newdirection_2)
  (bind _output_get (set `self.Rotation` (`KismetMathLibrary.MakeRotFromXY` (`self.DrX`) (`self.DrY`))))
  (return _output_get))

(fn `PortalConvertVelocity`
  (params (CurrentPortal :type "Actor Object Reference") (TargetPortal :type "Actor Object Reference") (PrevVelocity :type "Vector Structure"))
  (returns (NewVelocity :type "Vector Structure"))
  (set `self.VelocitySize` (`KismetMathLibrary.VSize` PrevVelocity))
  (bind _newdirection (`self.PortalConvertDirection` CurrentPortal TargetPortal (`KismetMathLibrary.Normal` PrevVelocity)))
  (set `self.VelocityDirection` _newdirection)
  (bind _output_get (set `self.Velocity` (* (`self.VelocityDirection`) (`self.VelocitySize`))))
  (return _output_get))

(fn `UserConstructionScript`)
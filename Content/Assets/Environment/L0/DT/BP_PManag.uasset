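; BP_PManag manages a linked pair of teleport points, P1 and P2, sending a player between them.
; Its Teleportation event takes the current point and moves the player to the other point's root location and rotation.
; A shared CanTeleport flag blocks further teleports during a short delay after each jump, then re-enables them.
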(event `Teleportation`
  (params (Current :type "/Game/Assets/Environment/L0/DT/BP_Portal Object Reference") (Player :type "Actor Object Reference"))
  (bind (_returnvalue_location _returnvalue_rotation) (`KismetMathLibrary.BreakTransform` (`SceneComponent.K2_GetComponentToWorld` (`/Game/Assets/Environment/L0/DT/BP_Portal.DefaultSceneRoot` (`self.P1`)))))
  (bind (_returnvalue_location_2 _returnvalue_rotation_2) (`KismetMathLibrary.BreakTransform` (`SceneComponent.K2_GetComponentToWorld` (`/Game/Assets/Environment/L0/DT/BP_Portal.DefaultSceneRoot` (`self.P2`)))))
  (if (`self.CanTeleport`)
    (if (== Current (`self.P1`))
      (set `self.CanTeleport` false)
      (`self.K2_SetActorTransform` Player (`KismetMathLibrary.MakeTransform` _returnvalue_location_2 _returnvalue_rotation_2) false false)
      (`KismetSystemLibrary.Delay` 0.5)
      (set `self.CanTeleport` true)
      (elif (== Current (`self.P2`))
        (set `self.CanTeleport` false)
        (`self.K2_SetActorTransform` Player (`KismetMathLibrary.MakeTransform` _returnvalue_location _returnvalue_rotation) false false)
        (`KismetSystemLibrary.Delay` 0.5)
        (set `self.CanTeleport` true)))))

(fn `UserConstructionScript`)
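; Level L0 gate that slides open once both referenced activators, PP1 and PP2, are active.
; Tick polls both Active flags and, after a Delay, plays two Timelines that move the left and right groups of gate cubes along relative Y.
; Each left Timeline update also sets Open to true and calls GateOpened on ShaderGate.
; A DoOnce follows the Timelines in the sequence but gates nothing.
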(event `self.ReceiveBeginPlay`
  (set `self.Open` false))

(event `self.ReceiveTick`
  (params (DeltaSeconds :type "Float (single-precision)"))
  (if (and (`/Game/ThirdPersonBP/Blueprints/L0/PressurePlate1_L0.Active` (`self.PP1`)) (`/Game/ThirdPersonBP/Blueprints/L0/PressurePlate2_L0.Active` (`self.PP2`)))
    (`KismetSystemLibrary.Delay` 4.0)
    (`|ExecutionSequence`
      (:`then_0`
        (`|ExecutionSequence`
          (:`then_0`
            (bind (_direction _newtrack_0) (`Timeline|LeftTimeline`)
              (:`Update`
                (`SceneComponent.K2_SetRelativeLocation` (`self.gate_Cube_008`) (`KismetMathLibrary.MakeVector` 0.0 _newtrack_0) false false)
                (`SceneComponent.K2_SetRelativeLocation` (`self.gate_Cube_013`) (`KismetMathLibrary.MakeVector` 0.0 _newtrack_0) false false)
                (`SceneComponent.K2_SetRelativeLocation` (`self.gate_Cube_020`) (`KismetMathLibrary.MakeVector` 0.0 _newtrack_0) false false)
                (`SceneComponent.K2_SetRelativeLocation` (`self.gate_Cube_012`) (`KismetMathLibrary.MakeVector` 0.0 _newtrack_0) false false)
                (`SceneComponent.K2_SetRelativeLocation` (`self.gate_Cube_019`) (`KismetMathLibrary.MakeVector` 0.0 _newtrack_0) false false)
                (`SceneComponent.K2_SetRelativeLocation` (`self.gate_Cube`) (`KismetMathLibrary.MakeVector` 0.0 _newtrack_0) false false)
                (`SceneComponent.K2_SetRelativeLocation` (`self.gate_Cube_014`) (`KismetMathLibrary.MakeVector` 0.0 _newtrack_0) false false)
                (`SceneComponent.K2_SetRelativeLocation` (`self.gate_Cube_015`) (`KismetMathLibrary.MakeVector` 0.0 _newtrack_0) false false)
                (`SceneComponent.K2_SetRelativeLocation` (`self.gate_Cube_036`) (`KismetMathLibrary.MakeVector` 0.0 _newtrack_0) false false)
                (`SceneComponent.K2_SetRelativeLocation` (`self.gate_Cube_034`) (`KismetMathLibrary.MakeVector` 0.0 _newtrack_0) false false)
                (`SceneComponent.K2_SetRelativeLocation` (`self.gate_Cube_023`) (`KismetMathLibrary.MakeVector` 0.0 _newtrack_0) false false)
                (`SceneComponent.K2_SetRelativeLocation` (`self.gate_Cube_002`) (`KismetMathLibrary.MakeVector` 0.0 _newtrack_0) false false)
                (`SceneComponent.K2_SetRelativeLocation` (`self.gate_Cube_007`) (`KismetMathLibrary.MakeVector` 0.0 _newtrack_0) false false)
                (`SceneComponent.K2_SetRelativeLocation` (`self.gate_Cube_024`) (`KismetMathLibrary.MakeVector` 0.0 _newtrack_0) false false)
                (`SceneComponent.K2_SetRelativeLocation` (`self.gate_Cube_029`) (`KismetMathLibrary.MakeVector` 0.0 _newtrack_0) false false)
                (`SceneComponent.K2_SetRelativeLocation` (`self.gate_Cube_032`) (`KismetMathLibrary.MakeVector` 0.0 _newtrack_0) false false)
                (`SceneComponent.K2_SetRelativeLocation` (`self.gate_Cube_028`) (`KismetMathLibrary.MakeVector` 0.0 _newtrack_0) false false)
                (set `self.Open` true)
                (`/Game/Assets/Shaders/Gate/BP_ShaderGate.GateOpened` (`self.ShaderGate`)))))
          (:`then_1`
            (bind (_direction_2 _rigthtimeline) (`Timeline|Timeline_0`)
              (:`Update`
                (`SceneComponent.K2_SetRelativeLocation` (`self.gate_Cube_033`) (`KismetMathLibrary.MakeVector` 0.0 _rigthtimeline) false false)
                (`SceneComponent.K2_SetRelativeLocation` (`self.gate_Cube_006`) (`KismetMathLibrary.MakeVector` 0.0 _rigthtimeline) false false)
                (`SceneComponent.K2_SetRelativeLocation` (`self.gate_Cube_010`) (`KismetMathLibrary.MakeVector` 0.0 _rigthtimeline) false false)
                (`SceneComponent.K2_SetRelativeLocation` (`self.gate_Cube_031`) (`KismetMathLibrary.MakeVector` 0.0 _rigthtimeline) false false)
                (`SceneComponent.K2_SetRelativeLocation` (`self.gate_Cube_004`) (`KismetMathLibrary.MakeVector` 0.0 _rigthtimeline) false false)
                (`SceneComponent.K2_SetRelativeLocation` (`self.gate_Cube_016`) (`KismetMathLibrary.MakeVector` 0.0 _rigthtimeline) false false)
                (`SceneComponent.K2_SetRelativeLocation` (`self.gate_Cube_009`) (`KismetMathLibrary.MakeVector` 0.0 _rigthtimeline) false false)
                (`SceneComponent.K2_SetRelativeLocation` (`self.gate_Cube_017`) (`KismetMathLibrary.MakeVector` 0.0 _rigthtimeline) false false)
                (`SceneComponent.K2_SetRelativeLocation` (`self.gate_Cube_035`) (`KismetMathLibrary.MakeVector` 0.0 _rigthtimeline) false false)
                (`SceneComponent.K2_SetRelativeLocation` (`self.gate_Cube_027`) (`KismetMathLibrary.MakeVector` 0.0 _rigthtimeline) false false)
                (`SceneComponent.K2_SetRelativeLocation` (`self.gate_Cube_005`) (`KismetMathLibrary.MakeVector` 0.0 _rigthtimeline) false false)
                (`SceneComponent.K2_SetRelativeLocation` (`self.gate_Cube_011`) (`KismetMathLibrary.MakeVector` 0.0 _rigthtimeline) false false)
                (`SceneComponent.K2_SetRelativeLocation` (`self.gate_Cube_018`) (`KismetMathLibrary.MakeVector` 0.0 _rigthtimeline) false false)
                (`SceneComponent.K2_SetRelativeLocation` (`self.gate_Cube_025`) (`KismetMathLibrary.MakeVector` 0.0 _rigthtimeline) false false)
                (`SceneComponent.K2_SetRelativeLocation` (`self.gate_Cube_022`) (`KismetMathLibrary.MakeVector` 0.0 _rigthtimeline) false false)
                (`SceneComponent.K2_SetRelativeLocation` (`self.gate_Cube_026`) (`KismetMathLibrary.MakeVector` 0.0 _rigthtimeline) false false)
                (`SceneComponent.K2_SetRelativeLocation` (`self.gate_Cube_003`) (`KismetMathLibrary.MakeVector` 0.0 _rigthtimeline) false false)
                (`SceneComponent.K2_SetRelativeLocation` (`self.gate_Cube_037`) (`KismetMathLibrary.MakeVector` 0.0 _rigthtimeline) false false)
                (`SceneComponent.K2_SetRelativeLocation` (`self.gate_Cube_030`) (`KismetMathLibrary.MakeVector` 0.0 _rigthtimeline) false false)
                (`SceneComponent.K2_SetRelativeLocation` (`self.gate_Cube_021`) (`KismetMathLibrary.MakeVector` 0.0 _rigthtimeline) false false))))))
      (:`then_1`
        (`/Engine/EditorBlueprintResources/StandardMacros.DoOnce` false)))))

(fn `UserConstructionScript`)
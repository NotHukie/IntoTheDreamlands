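; Level 2 interior environment actor that animates its exit doors and closes its entry doors.
; A custom event plays the Exit timeline, sliding two TentDoors meshes apart in opposite directions along X.
; The same timeline moves FTMesa toward a fixed X, lerping from its current position each update.
; CloseEntry instantly snaps the other two door meshes back to their zero relative location.
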(event `CustomEvent_0`
  (bind _ftmesa (`self.FTMesa`))
  (bind (_relativelocation_x _relativelocation_y _relativelocation_z) (`KismetMathLibrary.BreakVector` (`SceneComponent.RelativeLocation` _ftmesa)))
  (bind (_direction _newtrack_0) (`Timeline|Exit` :!via `PlayFromStart`)
    (:`Update`
      (bind _returnvalue (`KismetMathLibrary.VLerp` (0.0 0.0 0.0) (145.0 0.0 0.0) _newtrack_0))
      (`SceneComponent.K2_SetRelativeLocation` (`self.TentDoors_Cube_015`) _returnvalue false false)
      (`SceneComponent.K2_SetRelativeLocation` (`self.TentDoors_Cube_013`) (* _returnvalue -1) false false)
      (`SceneComponent.K2_SetRelativeLocation` _ftmesa (`KismetMathLibrary.VLerp` (`KismetMathLibrary.MakeVector` _relativelocation_x _relativelocation_y _relativelocation_z) (`KismetMathLibrary.MakeVector` 250.0 _relativelocation_y _relativelocation_z) _newtrack_0) false false))))

(fn `CloseEntry`
  (`SceneComponent.K2_SetRelativeLocation` (`self.TentDoors_Cube_017`) (0.0 0.0 0.0) false false)
  (`SceneComponent.K2_SetRelativeLocation` (`self.TentDoors_Cube_012`) (0.0 0.0 0.0) false false))

(fn `UserConstructionScript`)
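; Tea cup ride environment actor for L2 that sets eight cups spinning when play begins.
; BeginPlay points the AllRotating movement component at the Empty component to rotate it as a whole.
; It pairs each cup with its own rotating movement component by array index and gives it a random single-axis spin rate.
; The movement components drive all motion, so Tick stays empty.
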(event `self.ReceiveBeginPlay`
  (bind _output_get (set `self.Cups` (`|MakeArray` (`self.TCR_Cup6`) (`self.TCR_Cup5`) (`self.TCR_Cup7`) (`self.TCR_Cup4`) (`self.TCR_Cup`) (`self.TCR_Cup3`) (`self.TCR_Cup2`) (`self.TCR_Cup1`))))
  (bind _output_get_2 (set `self.RotaterCups` (`|MakeArray` (`self.CupsRotating1`) (`self.CupsRotating2`) (`self.CupsRotating3`) (`self.CupsRotating4`) (`self.CupsRotating5`) (`self.CupsRotating6`) (`self.CupsRotating7`) (`self.CupsRotating`))))
  (`MovementComponent.SetUpdatedComponent` (`self.AllRotating`) (`self.Empty`))
  (for (_array_element _array_index) _output_get
    (bind _output (`|GetArrayItem` _output_get_2 _array_index))
    (`MovementComponent.SetUpdatedComponent` _output _array_element)
    (set `RotatingMovementComponent.RotationRate` (`KismetMathLibrary.MakeRotator` 0.0 0.0 (`KismetMathLibrary.RandomFloatInRange` 5.0 20.0)) _output)))

(event `self.ReceiveTick`
  (params (DeltaSeconds :type "Float (single-precision)")))

(fn `UserConstructionScript`)
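; Portal manager that teleports the player between two linked portals, P1 and P2.
; Teleportation and ExitTeleport receive the current portal and move the player to an offset from the other, flipping yaw when arriving at P2.
; On arrival at P1, Teleportation adopts the portal's rotation, while ExitTeleport keeps the player's rotation and positions from PortalMesh1.
; A shared CanTeleport flag with a short delay prevents immediate re-teleporting.
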(event `Teleportation`
  (params (Current :type "Actor Object Reference") (Player :type "Actor Object Reference"))
  (bind _returnvalue (`SceneComponent.K2_GetComponentToWorld` (`/Game/Assets/Environment/L2/DT/BP_Portal_3.DefaultSceneRoot` (`self.P2`))))
  (bind (_returnvalue_location _returnvalue_rotation) (`KismetMathLibrary.BreakTransform` (`SceneComponent.K2_GetComponentToWorld` (`/Game/Assets/Environment/L2/DT/BP_Portal_2.DefaultSceneRoot` (`self.P1`)))))
  (if (`self.CanTeleport`)
    (if (== Current (`self.P1`))
      (set `self.CanTeleport` false)
      (`self.K2_SetActorTransform` Player (`KismetMathLibrary.MakeTransform` (+ (.location _returnvalue) (200.0 100.0 0.0)) (`KismetMathLibrary.MakeRotator` (.roll (.rotation _returnvalue)) (.pitch (.rotation _returnvalue)) (+ (.yaw (.rotation _returnvalue)) 180.0))) false false)
      (`KismetSystemLibrary.Delay` 0.5)
      (set `self.CanTeleport` true)
      (elif (== Current (`self.P2`))
        (set `self.CanTeleport` false)
        (`self.K2_SetActorTransform` Player (`KismetMathLibrary.MakeTransform` (+ _returnvalue_location (-50.0 0.0 0.0)) _returnvalue_rotation) false false)
        (`KismetSystemLibrary.Delay` 0.5)
        (set `self.CanTeleport` true)))))

(event `ExitTeleport`
  (params (Current :type "Actor Object Reference") (Player :type "Actor Object Reference"))
  (bind (_returnvalue_location _returnvalue_rotation) (`KismetMathLibrary.BreakTransform` (`SceneComponent.K2_GetComponentToWorld` (`Actor.RootComponent` Player))))
  (bind _returnvalue_location_2 (`KismetMathLibrary.BreakTransform` (`SceneComponent.K2_GetComponentToWorld` (`/Game/Assets/Environment/L2/DT/BP_Portal_2.PortalMesh1` (`self.P1`)))))
  (bind _returnvalue (`SceneComponent.K2_GetComponentToWorld` (`/Game/Assets/Environment/L2/DT/BP_Portal_3.DefaultSceneRoot` (`self.P2`))))
  (if (`self.CanTeleport`)
    (if (== Current (`self.P1`))
      (set `self.CanTeleport` false)
      (`self.K2_SetActorTransform` Player (`KismetMathLibrary.MakeTransform` (+ (.location _returnvalue) (200.0 100.0 0.0)) (`KismetMathLibrary.MakeRotator` (.roll (.rotation _returnvalue)) (.pitch (.rotation _returnvalue)) (+ (.yaw (.rotation _returnvalue)) 180.0))) false false)
      (`KismetSystemLibrary.Delay` 0.5)
      (set `self.CanTeleport` true)
      (elif (== Current (`self.P2`))
        (set `self.CanTeleport` false)
        (`self.K2_SetActorTransform` Player (`KismetMathLibrary.MakeTransform` (+ _returnvalue_location_2 (-50.0 0.0 0.0)) _returnvalue_rotation) false false)
        (`KismetSystemLibrary.Delay` 0.5)
        (set `self.CanTeleport` true)))))

(fn `UserConstructionScript`)
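; BP_GroundTube is an environment actor that animates the yaw of six tube ground cover components once play begins.
; Timeline_0 adds its track value to each cover's relative yaw on every update, zeroing roll and pitch.
; When it finishes, a five-second delay precedes Timeline_1, which applies the same incremental rotation.
; That second pass also targets the element reference left from the first loop.
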(event `self.ReceiveBeginPlay`
  (bind _output_get (set `self.CoverArray` (`|MakeArray` (`self.TubeGround_cover`) (`self.TubeGround_cover1`) (`self.TubeGround_cover2`) (`self.TubeGround_cover3`) (`self.TubeGround_cover4`) (`self.TubeGround_cover5`))))
  (bind (_direction _newtrack_3) (`Timeline|Timeline_0`)
    (:`Update`
      (for _array_element _output_get
        (`SceneComponent.K2_SetRelativeRotation` _array_element (`KismetMathLibrary.MakeRotator` 0.0 0.0 (+ (.yaw (.rotation (`SceneComponent.GetRelativeTransform` _array_element))) _newtrack_3)) false false)))
    (:`Finished`
      (`KismetSystemLibrary.Delay` 5.0)
      (bind (_direction_2 _newtrack_3_2) (`Timeline|Timeline_1`)
        (:`Update`
          (for _array_element_2 _output_get
            (`SceneComponent.K2_SetRelativeRotation` _array_element (`KismetMathLibrary.MakeRotator` 0.0 0.0 (+ (.yaw (.rotation (`SceneComponent.GetRelativeTransform` _array_element_2))) _newtrack_3_2)) false false)
            (`SceneComponent.K2_SetRelativeRotation` _array_element_2 (`KismetMathLibrary.MakeRotator` 0.0 0.0 (+ (.yaw (.rotation (`SceneComponent.GetRelativeTransform` _array_element_2))) _newtrack_3_2)) false false)))))))

(event `self.ReceiveTick`
  (params (DeltaSeconds :type "Float (single-precision)")))

(fn `UserConstructionScript`)
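; BP_TubeSmall is a ground tube with a hinged trap that takes in marshmallow pickups.
; The trap opens on BeginPlay, with timelines driving the Cube's pitch to open and close it.
; Any Trigger overlap closes the trap.
; If the overlapping actor casts to BP_MarshmallowPickUp, it calls GoUp on the Marshmallow reference and AttachToGroundTube on the pickup.
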(event `self.ReceiveBeginPlay`
  (`self.OpenTrap`))

(event `self.Trigger.OnComponentBeginOverlap`
  (params (OverlappedComponent :type "PrimitiveComponent Object Reference") (OtherActor :type "Actor Object Reference") (OtherComp :type "PrimitiveComponent Object Reference") (OtherBodyIndex :type Integer) (bFromSweep :type Boolean) (SweepResult :type "HitResult Structure (by ref)"))
  (`self.CloseTrap`)
  (for _array_element (`Actor.Tags` OtherActor)
    (if (== _array_element "Marshmallow")
      (break)))
  (bind _asbp_marshmallow_pick_up (cast `/Game/Assets/Environment/TubeGround/BP_MarshmallowPickUp` OtherActor))
  (`/Game/ThirdPersonBP/Blueprints/ChocoPlat.GoUp` (`self.Marshmallow`) self)
  (`/Game/Assets/Environment/TubeGround/BP_MarshmallowPickUp.AttachToGroundTube` _asbp_marshmallow_pick_up))

(event `OpenTrap`
  (bind (_direction _newtrack_1) (`Timeline|Timeline_0` :!via `PlayFromStart`)
    (:`Update`
      (`SceneComponent.K2_SetRelativeRotation` (`self.Cube`) (`KismetMathLibrary.MakeRotator` 0.0 _newtrack_1) false false))))

(event `CloseTrap`
  (bind (_direction _newtrack_1) (`Timeline|Timeline_1` :!via `PlayFromStart`)
    (:`Update`
      (`SceneComponent.K2_SetRelativeRotation` (`self.Cube`) (`KismetMathLibrary.MakeRotator` 0.0 _newtrack_1) false false))))

(fn `UserConstructionScript`)
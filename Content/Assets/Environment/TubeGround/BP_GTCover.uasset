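; BP_GTCover is a TubeGround cover actor that swings open and closed by rotating its TubeGroundCover component around yaw.
; OpenCover and CloseCover events each play their own timeline from the start, respectively adding or subtracting the track value from the current relative yaw.
; The rotation accumulates on every timeline update, so the total swing depends on update count, and each update zeroes pitch and roll.
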(event `self.ReceiveBeginPlay`)

(event `OpenCover`
  (bind _tubeground_cover (`self.TubeGround_cover`))
  (bind (_direction _newtrack_0) (`Timeline|Timeline_0` :!via `PlayFromStart`)
    (:`Update`
      (`SceneComponent.K2_SetRelativeRotation` _tubeground_cover (`KismetMathLibrary.MakeRotator` 0.0 0.0 (+ (.yaw (.rotation (`SceneComponent.GetRelativeTransform` _tubeground_cover))) _newtrack_0)) false false))))

(event `CloseCover`
  (bind _tubeground_cover (`self.TubeGround_cover`))
  (bind (_direction _newtrack_0) (`Timeline|Timeline_1` :!via `PlayFromStart`)
    (:`Update`
      (`SceneComponent.K2_SetRelativeRotation` _tubeground_cover (`KismetMathLibrary.MakeRotator` 0.0 0.0 (- (.yaw (.rotation (`SceneComponent.GetRelativeTransform` _tubeground_cover))) _newtrack_0)) false false))))

(fn `UserConstructionScript`)
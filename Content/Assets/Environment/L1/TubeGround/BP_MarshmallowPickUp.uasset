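; Marshmallow pickup Blueprint that presents itself from a ground tube.
; Three seconds after BeginPlay, it opens the referenced GroundTube and attaches to the SpawnPoint socket on its first child component, keeping world scale.
; Overlap events defer to the parent class.
; PickUp is empty; logic for binding the player's Interact input and closing the tube on pickup is disconnected.
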(event `Pick Up`)

(event `Pick Up Pressed`
  (`self.PickUpPressed`))

(event `self.ReceiveBeginPlay`
  (`KismetSystemLibrary.Delay` 3.0)
  (`self.AttachToGroundTube`))

(event `self.ReceiveActorBeginOverlap`
  (params (OtherActor :type "Actor Object Reference"))
  (`parent.ReceiveActorBeginOverlap` OtherActor))

(event `self.ReceiveActorEndOverlap`
  (params (OtherActor :type "Actor Object Reference"))
  (`parent.ReceiveActorEndOverlap` OtherActor))

(fn `AttachToGroundTube`
  (`/Game/Assets/Environment/L1/TubeGround/BP_GroundTube.Open` (`self.GroundTube_0`))
  (`self.K2_AttachToComponent` (`SceneComponent.GetChildComponent` (`Actor.RootComponent` (`self.GroundTube_0`)) 0) "SpawnPoint" "SnapToTarget" "SnapToTarget" "KeepWorld"))

(fn `UserConstructionScript`)
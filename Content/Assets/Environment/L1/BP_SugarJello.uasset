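; BP_SugarJello is a Level 1 environment sugar object that bounces with a jello-style reaction on impact.
; When Sugar's hit involves a component tagged Bounce, it gets a strong upward impulse.
; The impact point goes into the PC_Data material parameter collection, and a timeline curve scaled by Itensity animates the impact normal there.
; Because the collection is global, each new hit overwrites the shared Location and Normal.
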(event `self.ReceiveTick`
  (params (DeltaSeconds :type "Float (single-precision)")))

(event `self.Sugar.OnComponentHit`
  (params (HitComponent :type "PrimitiveComponent Object Reference") (OtherActor :type "Actor Object Reference") (OtherComp :type "PrimitiveComponent Object Reference") (NormalImpulse :type "Vector Structure") (Hit :type "HitResult Structure (by ref)"))
  (bind (_bblockinghit _binitialoverlap _time _distance _location _impactpoint _normal _impactnormal _physmat _hitactor _hitcomponent) (`GameplayStatics.BreakHitResult` Hit))
  ;[1 1 1] Jello
  (if (`ActorComponent.ComponentHasTag` _hitcomponent "Bounce")
    (`PrimitiveComponent.AddImpulse` (`self.Sugar`) (0.0 0.0 250000.0) "None" false)
    (`KismetMaterialLibrary.SetVectorParameterValue` "/Game/Assets/Shaders/JelloLacke/PC_Data.PC_Data" "Location" (`KismetMathLibrary.Conv_VectorToLinearColor` _impactpoint))
    (bind (_direction _cu_bounce_tut) (`Timeline|Timeline_0` :!via `PlayFromStart`)
      (:`Update`
        (`KismetMaterialLibrary.SetVectorParameterValue` "/Game/Assets/Shaders/JelloLacke/PC_Data.PC_Data" "Normal" (`KismetMathLibrary.Conv_VectorToLinearColor` (* _impactnormal (* _cu_bounce_tut (`self.Itensity`)))))))))

(fn `UserConstructionScript`)